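; Non-playable character pawn that can follow or pursue and attack a target actor supplied through TargetAcquire.
; AIFollow and AIPursuit are self-looping events that re-issue AIMoveTo after a FollowDelay, with follow ending once very close to the target.
; In close range, pursuit calls AIAttack, which sends AttackMessage to the Weapon child actor and sets CharacterStates, reset after each delay.
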(event `AIFollow`
  (bind _targetactor (`self.TargetActor`))
  (`/Engine/EditorBlueprintResources/StandardMacros.IsValid` _targetactor
    (:`Is Valid`
      (if (not (< (`KismetMathLibrary.Vector_Distance` (`self.K2_GetActorLocation`) (`self.K2_GetActorLocation` _targetactor)) 5.0)) :!label _label
        (`|AIMoveTo` self (0.0 0.0 0.0) _targetactor 1.0
          (:`then`
            (`KismetSystemLibrary.Delay` (`self.FollowDelay`))
            (goto _label)))))))

(event `AIPursuit`
  (bind _targetactor (`self.TargetActor`))
  (`/Engine/EditorBlueprintResources/StandardMacros.IsValid` _targetactor
    (:`Is Valid`
      (if (< (`KismetMathLibrary.Vector_Distance` (`self.K2_GetActorLocation`) (`self.K2_GetActorLocation` _targetactor)) 150.0) :!label _label_2
        (`self.AIAttack`)
        (else
          (`|AIMoveTo` self (0.0 0.0 0.0) _targetactor 1.0
            (:`then`
              _))))
      (`KismetSystemLibrary.Delay` (`self.FollowDelay`))
      (set `self.CharacterStates` "NewEnumerator0")
      (goto _label_2))))

(event `TargetAcquire`
  (params (TargetActor :type "Actor Object Reference"))
  (set `self.TargetActor` TargetActor))

(event `AIAttack`
  (message `/Game/Blueprints/Interfaces/IWeapon.Attack` (`ChildActorComponent.ChildActor` (`self.Weapon`)))
  (set `self.CharacterStates` "NewEnumerator1"))

(fn `UserConstructionScript`)