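; BP_MeleeWeapon is a melee weapon actor that damages characters it touches during an attack.
; Its owner is set through SetOwningCharacter, and Attack arms it by setting an IsAttacking flag.
; When its Box overlaps an actor implementing ICharacter other than the owner, it sends a damage message and disarms, so each attack lands at most one hit.
; The flag clears only on a hit, so a missed attack leaves it armed.
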(event `/Game/Blueprints/Interfaces/IWeapon.SetOwningCharacter`
  (params (Character :type "/Game/Blueprints/Interfaces/ICharacter Interface"))
  (bind _asbp_character (cast `/Game/Blueprints/Pawns/BP_Character` Character))
  (set `self.OwningCharacter` _asbp_character))

(event `/Game/Blueprints/Interfaces/IWeapon.Attack`
  (set `self.bIsAttacking` true))

(event `self.Box.OnComponentBeginOverlap`
  (params (OverlappedComponent :type "PrimitiveComponent Object Reference") (OtherActor :type "Actor Object Reference") (OtherComp :type "PrimitiveComponent Object Reference") (OtherBodyIndex :type Integer) (bFromSweep :type Boolean) (SweepResult :type "HitResult Structure (by ref)"))
  (if (`self.bIsAttacking`)
    (if (`KismetSystemLibrary.DoesImplementInterface` OtherActor "/Game/Blueprints/Interfaces/ICharacter.ICharacter_C")
      (if (!= OtherActor (`self.OwningCharacter`))
        (message `/Game/Blueprints/Interfaces/ICharacter.TakeDamage` OtherActor 20.0)
        (set `self.bIsAttacking` false)))))

(fn `UserConstructionScript`)