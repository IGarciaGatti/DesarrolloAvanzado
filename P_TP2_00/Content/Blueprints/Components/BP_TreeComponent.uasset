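; BP_TreeComponent is a component that presents branching dialogue or decision options to the player through an on-screen panel.
; It creates WBP_DecisionPanel on BeginPlay and binds its button press to SelectOption.
; ReceiveOptions stores the given options, shows them and switches to UI input with the cursor visible.
; SelectOption restores game-only input and only prints a Peace or War score message for the chosen branch.
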(event `self.ReceiveBeginPlay`
  (bind _returnvalue (`|CreateWidget` "/Game/Blueprints/WidgetBPs/WBP_DecisionPanel.WBP_DecisionPanel_C" (`GameplayStatics.GetPlayerController` 0)))
  (bind _output_get (set `self.HUD` _returnvalue))
  (`UserWidget.AddToViewport` _output_get 0)
  (add `/Game/Blueprints/WidgetBPs/WBP_DecisionPanel.OnButtonPressed` (`self.HUD`) (delegate `SelectOption`)))

(event `SelectOption`
  (params (ButtonIndex :type Integer))
  (bind _returnvalue (`GameplayStatics.GetPlayerController` 0))
  (`WidgetBlueprintLibrary.SetInputMode_GameOnly` _returnvalue)
  (set `PlayerController.bShowMouseCursor` false _returnvalue)
  (switch `/Game/Blueprints/Enums/EBranches` (`.Branch_12_0C2B20C84B15D2FCEFB0F28A9055EE3C` (break `/Game/Blueprints/Structs/BranchOption` (`|GetArrayItem` (`self.CurrentOptions`) ButtonIndex)))
    (:`NewEnumerator0`
      (`KismetSystemLibrary.PrintString` "+10 Pacífico"))
    (:`NewEnumerator1`
      (`KismetSystemLibrary.PrintString` "+10 Violento" true true (struct :`R` 1.0 :`B` 0.017848 :`A` 1.0)))))

(event `ReceiveOptions`
  (params (Options :type "Array of /Game/Blueprints/Structs/BranchOption Structure"))
  (bind _returnvalue (`GameplayStatics.GetPlayerController` 0))
  (set `self.CurrentOptions` Options)
  (`WidgetBlueprintLibrary.SetInputMode_GameAndUIEx` _returnvalue (`self.HUD`) "LockAlways" false)
  (set `PlayerController.bShowMouseCursor` true _returnvalue)
  (`/Game/Blueprints/WidgetBPs/WBP_DecisionPanel.ShowOptions` (`self.HUD`) Options))