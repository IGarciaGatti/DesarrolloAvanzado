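; BP_HealthComponent is a component that tracks its owner's health and death state.
; AlterHealth adds a signed value to CurrentHealth while the owner is alive, then runs CheckDeath.
; CheckDeath fires OnDeath and sets IsDead once health reaches MinHealth or below, so later changes are ignored.
; The shown logic applies no upper clamp to health.
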(event `AlterHealth`
  (params (Value :type "Float (double-precision)"))
  (if (not (`self.bIsDead`))
    (set `self.CurrentHealth` (+ (`self.CurrentHealth`) Value))
    (`self.CheckDeath`)))

(event `CheckDeath`
  (if (<= (`self.CurrentHealth`) (`self.MinHealth`))
    (`self.OnDeath`)
    (set `self.bIsDead` true)))